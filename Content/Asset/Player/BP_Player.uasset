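; BP_Player is the player Blueprint that passes body key point positions to its skeletal mesh's animation Blueprint, ABP_Player.
; SetKeyPointPosition casts the mesh's anim instance, caches it, and copies positions for the pelvis, neck, head and both arm and leg chains into matching variables.
; The event graph holds no logic, so positions must come from an external caller, and their use in posing is left to ABP_Player.
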(event `self.ReceiveTick`
  (params (DeltaSeconds :type "Float (single-precision)")))

(fn `Set Key Point Position`
  (params (Pelvis_Position :type "Vector Structure") (Thigh_R_Position :type "Vector Structure") (Calf_R_Position :type "Vector Structure") (Foot_R_Position :type "Vector Structure") (Thigh_L_Position :type "Vector Structure") (Calf_L_Position :type "Vector Structure") (Foot_L_Position :type "Vector Structure") (Neck_Position :type "Vector Structure") (Head_Position :type "Vector Structure") (Upperarm_L_Position :type "Vector Structure") (Lowerarm_L_Position :type "Vector Structure") (Hand_L_Position :type "Vector Structure") (Upperarm_R_Position :type "Vector Structure") (Lowerarm_R_Position :type "Vector Structure") (Hand_R_Position :type "Vector Structure"))
  (bind _abp__player (`self.ABP_ Player`))
  (bind _asabp_player (cast `/Game/Asset/Player/ABP_Player` (`SkeletalMeshComponent.GetAnimInstance` (`self.Mesh`))))
  (set `self.ABP_ Player` _asabp_player)
  (`|ExecutionSequence`
    (:`then_0`
      (set `/Game/Asset/Player/ABP_Player.Pelvis Position` Pelvis_Position _abp__player))
    (:`then_1`
      (set `/Game/Asset/Player/ABP_Player.Thigh R Position` Thigh_R_Position _abp__player))
    (:`then_2`
      (set `/Game/Asset/Player/ABP_Player.Calf R Position` Calf_R_Position _abp__player))
    (:`then_3`
      (set `/Game/Asset/Player/ABP_Player.Foot R Position` Foot_R_Position _abp__player))
    (:`then_4`
      (set `/Game/Asset/Player/ABP_Player.Thigh L Position` Thigh_L_Position _abp__player))
    (:`then_5`
      (set `/Game/Asset/Player/ABP_Player.Calf L Position` Calf_L_Position _abp__player))
    (:`then_6`
      (set `/Game/Asset/Player/ABP_Player.Foot L Position` Foot_L_Position _abp__player))
    (:`then_7`
      (set `/Game/Asset/Player/ABP_Player.Neck Position` Neck_Position _abp__player))
    (:`then_8`
      (set `/Game/Asset/Player/ABP_Player.Head Position` Head_Position _abp__player))
    (:`then_9`
      (set `/Game/Asset/Player/ABP_Player.Upperarm L Position` Upperarm_L_Position _abp__player))
    (:`then_10`
      (set `/Game/Asset/Player/ABP_Player.Lowerarm L Position` Lowerarm_L_Position _abp__player))
    (:`then_11`
      (set `/Game/Asset/Player/ABP_Player.Hand L Position` Hand_L_Position _abp__player))
    (:`then_12`
      (set `/Game/Asset/Player/ABP_Player.Upperarm R Position` Upperarm_R_Position _abp__player))
    (:`then_13`
      (set `/Game/Asset/Player/ABP_Player.Lowerarm R Position` Lowerarm_R_Position _abp__player))
    (:`then_14`
      (set `/Game/Asset/Player/ABP_Player.Hand R Position` Hand_R_Position _abp__player))))

(fn `UserConstructionScript`
  (`parent.UserConstructionScript`))