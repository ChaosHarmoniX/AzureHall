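; BP_MainTask is an actor that relays body keypoint positions to the Player for posing a skeleton.
; SetPosition maps a joint index to named pelvis, leg, neck, head and arm vectors, skipping indices 7 and 8.
; Each Tick calls CallOnMainTask, pushes all stored joints through Player.SetKeyPointPosition, then calls QuitGame with no condition shown.
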(event `self.ReceiveBeginPlay`)

(event `self.ReceiveTick`
  (params (DeltaSeconds :type "Float (single-precision)"))
  (`self.OnMainTask`)
  (`/Game/Asset/Player/BP_Player.Set Key Point Position` (`self.Player`) (`self.Pelvis_Position`) (`self.Thigh_R_Position`) (`self.Calf_R_Position`) (`self.Foot_R_Position`) (`self.Thigh_L_Position`) (`self.Calf_L_Position`) (`self.Foot_L_Position`) (`self.Neck_Position`) (`self.Head_Position`) (`self.Upperarm_L_Position`) (`self.Lowerarm_L_Position`) (`self.Hand_L_Position`) (`self.Upperarm_R_Position`) (`self.Lowerarm_R_Position`) (`self.Hand_R_Position`))
  (`KismetSystemLibrary.QuitGame` null "Quit"))

(fn `SetPosition`
  (params (index :type Integer) (X :type "Float (double-precision)") (Y :type "Float (double-precision)") (Z :type "Float (double-precision)"))
  (bind _returnvalue (`KismetMathLibrary.MakeVector` X Y Z))
  (switch `int` index
    (:`0`
      (set `self.Pelvis_Position` _returnvalue))
    (:`1`
      (set `self.Thigh_R_Position` _returnvalue))
    (:`2`
      (set `self.Calf_R_Position` _returnvalue))
    (:`3`
      (set `self.Foot_R_Position` _returnvalue))
    (:`4`
      (set `self.Thigh_L_Position` _returnvalue))
    (:`5`
      (set `self.Calf_L_Position` _returnvalue))
    (:`6`
      (set `self.Foot_L_Position` _returnvalue))
    (:`9`
      (set `self.Neck_Position` _returnvalue))
    (:`10`
      (set `self.Head_Position` _returnvalue))
    (:`11`
      (set `self.Upperarm_L_Position` _returnvalue))
    (:`12`
      (set `self.Lowerarm_L_Position` _returnvalue))
    (:`13`
      (set `self.Hand_L_Position` _returnvalue))
    (:`14`
      (set `self.Upperarm_R_Position` _returnvalue))
    (:`15`
      (set `self.Lowerarm_R_Position` _returnvalue))
    (:`16`
      (set `self.Hand_R_Position` _returnvalue))))

(fn `UserConstructionScript`)